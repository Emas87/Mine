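; Player controller that streams BP_MC_Chunk voxel terrain around the controlled pawn on a flat XY grid.
; BeginPlay derives chunk size from the voxel settings and spawns the first chunks within a circular render range.
; Tick watches the pawn's rounded chunk coordinates and, on change, destroys out-of-range chunks and spawns missing ones with the controller's noise and material settings.
; Parallel arrays of coordinates and actor references track live chunks.
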(event `self.ReceiveBeginPlay`
  (bind (_x _y) (`self.GetPlayerChunkCoordinates`))
  (`self.Initialize`)
  (`self.SpawnNewChunksWithinRenderRange`)
  (set `self.LastKnownPlayerCoordinates` (make `IntVector` _x _y)))

(event `self.ReceiveTick`
  (params (DeltaSeconds :type "Float (single-precision)"))
  (bind (_x _y) (`self.GetPlayerChunkCoordinates`))
  (bind (_x_2 _y_2) (`self.GetPlayerChunkCoordinates`))
  (bind (_lastknownplayercoordinates_x _lastknownplayercoordinates_y) (break `IntVector` (`self.LastKnownPlayerCoordinates`)))
  (if (not (and (== _lastknownplayercoordinates_x _x) (== _y _lastknownplayercoordinates_y)))
    (set `self.LastKnownPlayerCoordinates` (make `IntVector` _x_2 _y_2))
    (`self.Player Has Changed Chunk Coordinates`)))

(event `Player Has Changed Chunk Coordinates`
  (`self.DestroyChunksOutsideREnderRange`)
  (`self.SpawnNewChunksWithinRenderRange`))

(fn `DestroyChunksOutsideREnderRange`
  (locals (IndexTemp :type Integer))
  (bind _chunk_size_xy (`self.Chunk Size XY`))
  (bind _indextemp (`local.IndexTemp`))
  (for (_array_element _array_index) (`self.CurrentSpawnedChunkCoordinates`)
    (set `local.IndexTemp` _array_index)
    (bind (_x _y _z) (break `IntVector` _array_element))
    (if (> (`KismetMathLibrary.Vector_Distance` (`KismetMathLibrary.MakeVector` (* _x _chunk_size_xy) (* _y _chunk_size_xy) (* _z _chunk_size_xy)) (`self.K2_GetActorLocation` (`self.K2_GetPawn`))) (* (`self.RenderRangeXYZ(Chunks)`) (`self.Chunk Size XY`)))
      (`self.K2_DestroyActor` (`|GetArrayItem` (`self.CurrentSpawnChunkReferences`) _indextemp))
      (`KismetArrayLibrary.Array_Remove` (`self.CurrentSpawnedChunkCoordinates`) _indextemp)
      (`KismetArrayLibrary.Array_Remove` (`self.CurrentSpawnChunkReferences`) _indextemp))))

(fn `GetPlayerChunkCoordinates`
  (returns (X :type Integer) (Y :type Integer))
  (return (`KismetMathLibrary.Round` (.x (/ (`self.K2_GetActorLocation` (`self.K2_GetPawn`)) (`self.Chunk Size XY`)))) (`KismetMathLibrary.Round` (.y (/ (`self.K2_GetActorLocation` (`self.K2_GetPawn`)) (`self.Chunk Size XY`))))))

(fn `Initialize`
  (set `self.Chunk Size XY` (* (* (`self.WithOfChunk(Voxels)`) 2) (`self.ChunkVoxelSize`))))

(fn `SpawnNewChunksWithinRenderRange`
  (locals (TempX :type Integer) (TempY :type Integer) (ChunkCoordinates :type "IntVector Structure") (TempZ :type Integer))
  (bind (_x _y) (`self.GetPlayerChunkCoordinates`))
  (bind _renderrangexyz_chunks_ (`self.RenderRangeXYZ(Chunks)`))
  (bind (_chunkcoordinates_x _chunkcoordinates_y _chunkcoordinates_z) (break `IntVector` (`local.ChunkCoordinates`)))
  (bind _renderrangexyz_chunks__2 (`self.RenderRangeXYZ(Chunks)`))
  (bind _chunk_size_xy (`self.Chunk Size XY`))
  (for _index (range (* _renderrangexyz_chunks_ -1) (+ _renderrangexyz_chunks_ 1))
    (set `local.TempX` _index)
    (for _index_2 (range (* _renderrangexyz_chunks__2 -1) (+ _renderrangexyz_chunks__2 1))
      (set `local.TempY` _index_2)
      (set `local.ChunkCoordinates` (make `IntVector` (+ _x (`local.TempX`)) (+ _y (`local.TempY`))))
      ;[1 1 1] Should Spawn a chunk?
      (if (and (not (`KismetArrayLibrary.Array_Contains` (`self.CurrentSpawnedChunkCoordinates`) (`local.ChunkCoordinates`))) (< (`KismetMathLibrary.VSize` (`KismetMathLibrary.MakeVector` (* (`local.TempX`) (`self.Chunk Size XY`)) (* (`local.TempY`) (`self.Chunk Size XY`)))) (* (`self.RenderRangeXYZ(Chunks)`) (`self.Chunk Size XY`))))
        ;[1 1 1] Spawn a new chunk at thi loops coordinates
        (bind _returnvalue (`|SpawnActorFromClass` "/Game/Blueprints/BP_MC_Chunk.BP_MC_Chunk_C" (`KismetMathLibrary.Conv_VectorToTransform` (`KismetMathLibrary.MakeVector` (* _chunkcoordinates_x _chunk_size_xy) (* _chunkcoordinates_y _chunk_size_xy) (* _chunkcoordinates_z _chunk_size_xy))) "DontSpawnIfColliding" "OverrideRootScale" null (`self.WithOfChunk(Voxels)`) (`self.DepthOfChunk(Voxels)`) (`self.ChunNoiseDensity`) (`self.ChunkNoiseScale(Voxels)`) (`self.MaterialTypes`) (`self.Chunk3dNoiseDensity`) (`self.Chunk3dNoiseCutOffBelowSurface`) (`self.Chunk Size XY`) (`self.Chunk Size XY`) (`self.ChunkVoxelSize`) null))
        (`KismetArrayLibrary.Array_Add` (`self.CurrentSpawnChunkReferences`) _returnvalue)
        (`KismetArrayLibrary.Array_Add` (`self.CurrentSpawnedChunkCoordinates`) (`local.ChunkCoordinates`))))))

(fn `UserConstructionScript`)