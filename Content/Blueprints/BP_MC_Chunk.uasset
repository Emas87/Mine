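; Voxel terrain chunk actor that builds a block landscape in its construction script, with no runtime logic.
; Creates one hierarchical instanced mesh component per material, then loops over the chunk's voxel grid.
; 2D simplex noise at world XY offsets each column's height, and 3D simplex noise carves gaps using separate surface and below-surface thresholds.
; Surviving voxels become snow, grass, dirt or rock instances by resulting height.
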(event `self.ReceiveBeginPlay`)

(fn `AddVoxelInstanceOfType(UsingWorldPos)`
  (params (ISMToAdd :type "InstancedStaticMeshComponent Object Reference"))
  (locals (Rotation :type "Rotator Structure"))
  (bind _voxeltrasnform (`self.GetVoxelTransform`)) ; Center of Voxel
  (`self.AddVoxel` _voxeltrasnform ISMToAdd))

(fn `Apply3dNoise`
  (params (CutOffThreshold :type "Float (double-precision)") (NoiseDensity :type "Float (double-precision)"))
  (returns (ShouldCutOff :type Boolean) (`3DNoiseDensity` :type "Float (double-precision)"))
  (bind _voxelsize (`self.VoxelSize`))
  (bind _returnvalue (`SimplexNoiseBPLibrary.SimplexNoise3D` (* (`self.WorldPosX`) _voxelsize) (* (`self.WorldPosY`) _voxelsize) (* (`self.WorldPosZ-PosNoise`) _voxelsize) NoiseDensity))
  (return (<= _returnvalue CutOffThreshold) 0.0))

(fn `GetVoxelTransform`
  (returns (VoxelTrasnform :type "Transform Structure"))
  (return (`KismetMathLibrary.MakeTransform` (`KismetMathLibrary.MakeVector` (* (`self.LocalVoxPosX`) (`self.VoxelSize`)) (* (`self.LocalVoxPosY`) (`self.VoxelSize`)) (* (`self.WorldPosZ-PosNoise`) (`self.VoxelSize`))) (struct) (* (1.0 1.0 1.0) (/ (`self.VoxelSize`) 100.0)))))

(fn `Initialize`
  (for _array_element (`self.MaterialTypes`)
    (bind _returnvalue (`AddComponent|NODE_AddHierarchicalInstancedStaticMeshComponent-1`))
    (`KismetArrayLibrary.Array_Add` (`self.ISMs`) _returnvalue)
    (`StaticMeshComponent.SetStaticMesh` _returnvalue "/Game/StaticMesh/Plane.Plane")
    (`PrimitiveComponent.SetMaterial` _returnvalue 0 _array_element)))

(fn `UserConstructionScript`
  (bind _num_2n_1_ (`self.Num(2n-1)`))
  (bind _num_2n_1__2 (`self.Num(2n-1)`))
  (bind _voxelsize (`self.VoxelSize`))
  (bind _depth (`self.Depth`))
  (`self.Initialize`)
  ;[1 1 1] Loops
  (for _index (range (* _num_2n_1_ -1) (+ _num_2n_1_ 1))
    (set `self.LocalVoxPosX` _index)
    (for _index_2 (range (* _num_2n_1__2 -1) (+ _num_2n_1__2 1))
      (set `self.LocalVoxPosY` _index_2)
      (for _index_3 (range (* _depth -1) (+ _depth 1))
        (set `self.LocalVoxPosZ` _index_3)
        ;[1 1 1] World Coordinates
        (set `self.WorldPosX` (+ (`self.LocalVoxPosX`) (`KismetMathLibrary.FFloor` (.x (/ (`self.K2_GetActorLocation`) (`self.VoxelSize`))))))
        (set `self.WorldPosY` (+ (`self.LocalVoxPosY`) (`KismetMathLibrary.FFloor` (.y (/ (`self.K2_GetActorLocation`) (`self.VoxelSize`))))))
        (set `self.WorldPosZ-PreNoise` (+ (`self.LocalVoxPosZ`) (`KismetMathLibrary.FFloor` (.z (/ (`self.K2_GetActorLocation`) (`self.VoxelSize`))))))
        ;[1 1 1] Calculate 2D Surface Noise
        (bind _returnvalue (`SimplexNoiseBPLibrary.SimplexNoise2D` (* (`self.WorldPosX`) _voxelsize) (* (`self.WorldPosY`) _voxelsize) (`self.NoiseDensity`)))
        (set `self.WorldPosZ-PosNoise` (- (`KismetMathLibrary.FFloor` (* (`self.NoiseScale`) _returnvalue)) (`self.LocalVoxPosZ`)))
        ;[1 1 1] Apply 3D Noise
        (if (>= (* (`self.LocalVoxPosZ`) -1) (- (`self.Depth`) 3))
          (bind _shouldcutoff (`self.Apply3dNoise` (`self.3dNoiseCutOffAtSurface`) (`self.3DNoiseDensity`)))
          (if (not _shouldcutoff)
            ;[1 1 1] Add ISM type depending on depth
            (if (> (`self.WorldPosZ-PosNoise`) 4) :!label _label
              (`self.AddVoxelInstanceOfType(UsingWorldPos)` (`|GetArrayItem` (`self.ISMs`))) ; Snow
              (elif (> (`self.WorldPosZ-PosNoise`) 2)
                (`self.AddVoxelInstanceOfType(UsingWorldPos)` (`|GetArrayItem` (`self.ISMs`) 1)) ; Grass
                (elif (> (`self.WorldPosZ-PosNoise`) 0)
                  (`self.AddVoxelInstanceOfType(UsingWorldPos)` (`|GetArrayItem` (`self.ISMs`) 2)) ; Dirt
                  (else
                    (`self.AddVoxelInstanceOfType(UsingWorldPos)` (`|GetArrayItem` (`self.ISMs`) 3)) ; Rock
                  )))))
          (else
            (bind _shouldcutoff_2 (`self.Apply3dNoise` (`self.3DNoiseCutoffBelowSurface`) (`self.3DNoiseDensity`)))
            (if (not _shouldcutoff_2)
              (goto _label))))))))